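; Player character for a grid-based game, with stepped movement, regenerating energy and spawned abilities.
; WASD teleports it one step within bounds set at spawn, after an optional slowdown delay toggled by right mouse.
; Events spawn ability actors at the billboard or a shadow clone; lane steal temporarily widens X bounds through Map_Grid and any clone.
; E spawns an enemy, Space spends energy, and several ability and UI chains are unwired.
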(event `self.ReceiveBeginPlay`
  (`|ExecutionSequence`
    (:`then_0`
      (`KismetSystemLibrary.K2_SetTimerDelegate` (delegate `FillEnergy`) 2.0 true))))

(event `FillEnergy`
  (if (< (`self.Energy`) 8.0)
    (bind _result (`/Engine/EditorBlueprintResources/StandardMacros.IncrementFloat` (`self.Energy`)))))

(event `spawn`
  (bind (_returnvalue_x _returnvalue_y) (`KismetMathLibrary.BreakVector` (`self.K2_GetActorLocation`)))
  (bind _max_minmovement (`self.Max&MInMovement`))
  ;[0.31 0.31 0.31] SpawnLocation
  (`self.K2_SetActorLocation` (`KismetMathLibrary.MakeVector` (`self.LocX`) (`self.LocY`)))
  (set `self.Maximum X` (+ _returnvalue_x _max_minmovement))
  (set `self.MinimumX` (- _returnvalue_x _max_minmovement))
  (set `self.Maximum Y` (+ _returnvalue_y _max_minmovement))
  (set `self.MinimumY` (- _returnvalue_y _max_minmovement)))

(event `Key|W`
  (params (Key :type "Key Structure" :default "AnyKey"))
  ;[0.007625 1 0.3544] Controls
  ;;[0.1824 0.08085 1] Movement Controls
  (:`Pressed`
    (set `self.Up` true)
    (set `self.Movement` -200.0)
    (if (`self.MovementEnable`) :!label _label
      (`KismetSystemLibrary.Delay` (`self.Slowdown`))
      (`self.Move`))))

(event `Key|E`
  (params (Key :type "Key Structure" :default "AnyKey"))
  (bind (_returnvalue_x _returnvalue_y _returnvalue_z) (`KismetMathLibrary.BreakVector` (`self.K2_GetActorLocation`)))
  (:`Pressed`
    (`|SpawnActorFromClass` "/Game/Game/Blueprints/Abilities/Enemy_Temporero.Enemy_Temporero_C" (`KismetMathLibrary.MakeTransform` (`KismetMathLibrary.MakeVector` (+ _returnvalue_x 600.0) _returnvalue_y _returnvalue_z)) "Undefined" "OverrideRootScale")))

(event `Key|S`
  (params (Key :type "Key Structure" :default "AnyKey"))
  ;[0.007625 1 0.3544] Controls
  ;;[0.1824 0.08085 1] Movement Controls
  (:`Pressed`
    (set `self.Up` true)
    (set `self.Movement` 200.0)
    (goto _label)))

(event `Move`
  (bind _returnvalue_x (`KismetMathLibrary.BreakVector` (`self.K2_GetActorLocation`)))
  (bind (_returnvalue_x_2 _returnvalue_y) (`KismetMathLibrary.BreakVector` (`self.K2_GetActorLocation`)))
  (bind _returnvalue (+ _returnvalue_y (`self.Movement`)))
  (bind _returnvalue_2 (+ _returnvalue_x (`self.Movement`)))
  ;[1 0 0.8355] Player Movement Action
  (if (`self.Up`)
    (if (not (or (< _returnvalue (`self.MinimumY`)) (> _returnvalue (`self.Maximum Y`))))
      (set `self.LocY` _returnvalue)
      (`self.K2_TeleportTo` (`KismetMathLibrary.MakeVector` (`self.LocX`) (`self.LocY`)) :!label _label_2))
    (elif (not (or (< _returnvalue_2 (`self.MinimumX`)) (> _returnvalue_2 (`self.Maximum X`))))
      (set `self.LocX` _returnvalue_2)
      (goto _label_2))))

(event `Back`
  ;[0.007625 1 0.3544] Controls
  ;;[0.1824 0.08085 1] Movement Controls
  (set `self.Up` false :!label _label_3)
  (set `self.Movement` -200.0)
  (goto _label))

(event `Key|A`
  (params (Key :type "Key Structure" :default "AnyKey"))
  ;[0.007625 1 0.3544] Controls
  ;;[0.1824 0.08085 1] Movement Controls
  (:`Pressed`
    (goto _label_3)))

(event `Key|D`
  (params (Key :type "Key Structure" :default "AnyKey"))
  ;[0.007625 1 0.3544] Controls
  ;;[0.1824 0.08085 1] Movement Controls
  (:`Pressed`
    (set `self.Up` false)
    (set `self.Movement` 200.0)
    (goto _label)))

(event `Clone`
  ;[1 1 1] Spawn Clone
  (set `self.Clone Active` true)
  (bind _returnvalue (`|SpawnActorFromClass` "/Game/Game/Blueprints/Abilities/ShadowClone_Ability.ShadowClone_Ability_C" (`KismetMathLibrary.MakeTransform` (`self.K2_GetActorLocation`)) "Undefined" "OverrideRootScale"))
  (`self.SetLifeSpan` _returnvalue 0.0))

(event `Abilities`
  (params (WhatAbility :type Text))
  (bind _returnvalue (`SceneComponent.K2_GetComponentLocation` (`self.Billboard`)))
  (set `self.Spawn Location` _returnvalue)
  (bind _returnvalue_2 (`|SpawnActorFromClass` "/Game/Game/Blueprints/Abilities/Abilities.Abilities_C" (`KismetMathLibrary.MakeTransform` _returnvalue) "Undefined" "OverrideRootScale"))
  (`/Game/Game/Blueprints/Abilities/Abilities.Activate` _returnvalue_2 WhatAbility))

(event `Lane`
  (bind _returnvalue_x (`KismetMathLibrary.BreakVector` (`self.K2_GetActorLocation`)))
  ;[1 0.1821 0.8166] Steal Lane
  (set `self.SteelLane` true)
  (`/Engine/EditorBlueprintResources/StandardMacros.DoOnce` false :!label _label_4
    (:`Completed`
      (if (`self.Clone Active`)
        ;;[1 1 1] add maximum x (Clone)
        (`/Game/Game/Blueprints/Abilities/ShadowClone_Ability.Add max mov x (steal lane)` (stale `Clone` _returnvalue)))
      (bind _outactors (`GameplayStatics.GetAllActorsOfClass` "/Game/Game/Blueprints/Grid_Programacion/Map_Grid.Map_Grid_C"))
      (`/Game/Game/Blueprints/Grid_Programacion/Map_Grid.Steal Lane` (`|GetArrayItem` _outactors))
      (set `self.Maximum X` (+ (`self.Maximum X`) (`self.Max&MInMovement`)))
      (`KismetSystemLibrary.Delay` 5.0)
      (set `self.Maximum X` (- (`self.Maximum X`) (`self.Max&MInMovement`)))
      (if (>= _returnvalue_x (+ (`self.Maximum X`) (`self.Max&MInMovement`)))
        (`self.Back`))
      ;;[1 1 1] If clone is active, move back
      (if (`self.Clone Active`)
        (`/Game/Game/Blueprints/Abilities/ShadowClone_Ability.Back Clone!` (stale `Clone` _returnvalue)))
      (`self.Reset`))))

(event `Reset`
  ;[1 0.1821 0.8166] Steal Lane
  (set `self.SteelLane` false)
  (goto _label_4 :!via `Reset`))

(event `Key|F`
  (params (Key :type "Key Structure" :default "AnyKey"))
  ;[1 1 1] Spawn Acha
)

(event `Key|G`
  (params (Key :type "Key Structure" :default "AnyKey"))
  ;[1 1 1] Spawn Infinite Laser
)

(event `Key|T`
  (params (Key :type "Key Structure" :default "AnyKey"))
  ;[1 1 1] Two Tile Spread Ability
)

(event `Key|RightMouseButton`
  (params (Key :type "Key Structure" :default "AnyKey"))
  ;[1 1 1] SlowDown Test
  (:`Pressed`
    (`/Engine/EditorBlueprintResources/StandardMacros.FlipFlop`
      (:`A`
        (set `self.Slowdown` 0.2))
      (:`B`
        (set `self.Slowdown` 0.0)))))

(event `ResetTtile`
  (bind _returnvalue (`SceneComponent.K2_GetComponentLocation` (`self.Billboard`)))
  ;[1 1 1] Two Tile Spread Ability
  (`/Engine/EditorBlueprintResources/StandardMacros.DoOnce` false :!via `Reset`
    (:`Completed`
      (set `self.Spawn Location` _returnvalue)
      (bind _returnvalue_2 (`|SpawnActorFromClass` "/Game/Game/Blueprints/Abilities/Abilities_JK.Abilities_JK_C" (`KismetMathLibrary.MakeTransform` _returnvalue) "Undefined" "OverrideRootScale"))
      (`/Game/Game/Blueprints/Abilities/Abilities_JK.TwoTileSpread` _returnvalue_2))))

(event `Key|SpaceBar`
  (params (Key :type "Key Structure" :default "AnyKey"))
  (:`Pressed`
    (`/Engine/EditorBlueprintResources/StandardMacros.DecrementFloat` (`self.Energy`))))

(fn `UserConstructionScript`)