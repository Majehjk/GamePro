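; BeginingGM is a Blueprint, apparently a game mode by its name, holding unused start-menu setup logic.
; Both EventGraph chains are disconnected from any event, so nothing in it runs.
; One chain, flagged for possible deletion, shows a StartMenu widget with game-and-UI input.
; The other checks for a save with an empty slot name and, if none exists, calls LoadCollection on BP_GameInstance and shows W_Main with cursor and UI-only input.
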(fn `UserConstructionScript`)