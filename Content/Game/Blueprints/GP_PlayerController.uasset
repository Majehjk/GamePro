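; Player controller that loads the local player's saved deck, requests a character spawn and brings up the main UI.
; On BeginPlay it clears widgets, reads the deck from the save slot and passes it to the server-side controller, where MapGM respawns the player.
; SetWidget then shows Start, loads the GameInstance collection after a delay and adds W_Main with mouse input.
; A looping one-second timer counts down minutes and seconds.
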(event `self.ReceiveBeginPlay`
  ;[1 1 1] Loads Players Deck and Passes info to Serverside Player Controller
  (if (`self.IsLocalController`)
    (`WidgetLayoutLibrary.RemoveAllWidgets`)
    (`self.LoadGame`)
    (`self.PassCharacterInfoToServer` (`self.PlayerDeckInfo`))))

(event `PassCharacterInfoToServer`
  (params (`Player Deck Info` :type "Array of /Game/Game/Structs/S_CardInfo Structure"))
  ;[1 1 1] Passes Character Deck info / Respawns Players with Selected Character
  (set `self.PlayerDeckInfo` `Player Deck Info`)
  (bind _asmap_gm (cast `/Game/Game/Blueprints/MapGM` (`GameplayStatics.GetGameMode`)))
  (`/Game/Game/Blueprints/MapGM.RespawnPlayer` _asmap_gm self "/Game/Game/Blueprints/Player/Player.Player_C") ; Character Needs change
  (`self.SetWidget`))

(event `SetWidget`
  (bind _returnvalue (`|CreateWidget` "/Game/Game/HUD/BatteMap/Start.Start_C"))
  (`UserWidget.AddToViewport` _returnvalue 0)
  (`KismetSystemLibrary.Delay` 1.0)
  (bind _asbp_game_instance (cast `/Game/Game/Blueprints/BP_GameInstance` (`GameplayStatics.GetGameInstance`)))
  (`/Game/Game/Blueprints/BP_GameInstance.LoadCollection` _asbp_game_instance)
  (set `PlayerController.bShowMouseCursor` true (`GameplayStatics.GetPlayerController` 0))
  (bind _returnvalue_2 (`|CreateWidget` "/Game/Game/HUD/W_Main.W_Main_C"))
  (bind _output_get (set `self.MainWidget` _returnvalue_2))
  (set `/Game/Game/Blueprints/BP_GameInstance.MainWidget` _output_get (cast `/Game/Game/Blueprints/BP_GameInstance` (`GameplayStatics.GetGameInstance`) :!pure true))
  (`UserWidget.AddToViewport` (`self.MainWidget`) 0)
  (`WidgetBlueprintLibrary.SetInputMode_GameAndUIEx` (`GameplayStatics.GetPlayerController` 0))
  (`KismetSystemLibrary.K2_SetTimerDelegate` (delegate `Timer`) 1.0 true))

(event `Timer`
  (if (== (`self.seconds`) 0)
    (`/Engine/EditorBlueprintResources/StandardMacros.DecrementInt` (`self.MIn`)
      (:`  `
        (set `self.seconds` 59)))
    (else
      (`/Engine/EditorBlueprintResources/StandardMacros.DecrementInt` (`self.seconds`)))))

(fn `LoadGame`
  (bind _returnvalue (`GameplayStatics.LoadGameFromSlot` (`self.PlayerSettingsSave`)))
  (bind _asplayer_save_game (cast `/Game/Game/HUD/Multiplayer/PlayerSaveGame` _returnvalue))
  (set `self.PlayerDeckInfo` (`/Game/Game/HUD/Multiplayer/PlayerSaveGame.S_PlayerDeck` _asplayer_save_game)))

(fn `UserConstructionScript`)