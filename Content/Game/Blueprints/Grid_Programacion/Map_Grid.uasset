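; Map_Grid is the battle grid actor, built from row and column tile components, that places the player and animates a lane steal.
; On BeginPlay it copies the F2C2 tile's world X and Y into the Player character, then calls its Spawn.
; StealLane sets materials on the three column-4 tiles, waits, then runs a looping timer whose Flicker FlipFlop reapplies materials before they are set a final time.
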(event `self.ReceiveBeginPlay`
  (bind (_returnvalue_x _returnvalue_y) (`KismetMathLibrary.BreakVector` (`SceneComponent.K2_GetComponentLocation` (`self.F2C2`))))
  ;[1 1 1] PlayerStart(BlueF2C2, RedF2C4)
  (bind _asplayer (cast `/Game/Game/Blueprints/Grid_Programacion/Player` (`GameplayStatics.GetPlayerCharacter` 0)))
  (set `/Game/Game/Blueprints/Grid_Programacion/Player.LocX` _returnvalue_x _asplayer)
  (set `/Game/Game/Blueprints/Grid_Programacion/Player.LocY` _returnvalue_y _asplayer)
  (`/Game/Game/Blueprints/Grid_Programacion/Player.spawn` _asplayer))

(event `Steal Lane`
  ;[0.4262 1 0.9701] Steal Lane Change color and Flicker
  (`PrimitiveComponent.SetMaterial` (`self.F1C4`) 0 null)
  (`PrimitiveComponent.SetMaterial` (`self.F3C4`) 0 null)
  (`PrimitiveComponent.SetMaterial` (`self.F2C4`) 0 null)
  (`KismetSystemLibrary.Delay` 3.0)
  (`KismetSystemLibrary.K2_SetTimer` self "Flicker" 0.2 true)
  (`KismetSystemLibrary.Delay` 2.0)
  (`KismetSystemLibrary.K2_ClearTimer` self "Flicker")
  (`PrimitiveComponent.SetMaterial` (`self.F1C4`) 0 null)
  (`PrimitiveComponent.SetMaterial` (`self.F3C4`) 0 null)
  (`PrimitiveComponent.SetMaterial` (`self.F2C4`) 0 null))

(event `Flicker`
  ;[0.4262 1 0.9701] Steal Lane Change color and Flicker
  (`/Engine/EditorBlueprintResources/StandardMacros.FlipFlop`
    (:`A`
      (`PrimitiveComponent.SetMaterial` (`self.F1C4`) 0 null)
      (`PrimitiveComponent.SetMaterial` (`self.F3C4`) 0 null)
      (`PrimitiveComponent.SetMaterial` (`self.F2C4`) 0 null))
    (:`B`
      (`PrimitiveComponent.SetMaterial` (`self.F2C4`) 0 null)
      (`PrimitiveComponent.SetMaterial` (`self.F3C4`) 0 null)
      (`PrimitiveComponent.SetMaterial` (`self.F1C4`) 0 null))))

(fn `UserConstructionScript`)