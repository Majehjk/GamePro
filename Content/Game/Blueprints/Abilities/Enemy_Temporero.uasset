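; Placeholder-style enemy clone that appears ahead of the player on X after a short delay and hops randomly around a bounded area.
; WhereToMove picks an axis and direction, then MoveClone teleports one fixed step, re-rolling when out of bounds and looping after a delay.
; StealLane.AddMaxMovX extends the forward X limit, while BackClone shrinks it and forces a backward step.
; Damage only lowers and prints Life, with no death handling.
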(event `self.ReceiveBeginPlay`
  (bind (_returnvalue_x _returnvalue_y) (`KismetMathLibrary.BreakVector` (`self.K2_GetActorLocation`)))
  (bind _max_minmovement (`self.Max&MInMovement`))
  (`KismetSystemLibrary.Delay` 0.5)
  (bind _asplayer (cast `/Game/Game/Blueprints/Player/Player` (`GameplayStatics.GetPlayerCharacter` 0)))
  (set `self.LocX` (+ (`/Game/Game/Blueprints/Player/Player.LocX` _asplayer) 600.0))
  (set `self.LocY` (`/Game/Game/Blueprints/Player/Player.LocY` _asplayer))
  (`self.K2_SetActorLocation` (`KismetMathLibrary.MakeVector` (`self.LocX`) (`self.LocY`)))
  (set `self.Maximum X` (+ _returnvalue_x _max_minmovement))
  (set `self.MinimumX` (- _returnvalue_x _max_minmovement))
  (set `self.Maximum Y` (+ _returnvalue_y _max_minmovement))
  (set `self.MinimumY` (- _returnvalue_y _max_minmovement))
  (`self.Where to move?`))

(event `Add max mov x (steal lane)`
  (set `self.Maximum X` (+ (`self.Maximum X`) (`self.Max&MInMovement`))))

(event `Back Clone!`
  (set `self.Up` false)
  (set `self.Maximum X` (- (`self.Maximum X`) (`self.Max&MInMovement`)))
  (set `self.Movement` -200.0 :!label _label)
  (`self.Move Clone` :!label _label_2))

(event `Where to move?`
  (bind _returnvalue (`KismetMathLibrary.RandomIntegerInRange` 1 2))
  (bind _output_get (set `self.Up` (`KismetMathLibrary.RandomBool`)))
  (if _output_get
    (if (== _returnvalue 1)
      (set `self.Movement` -200.0)
      (goto _label_2)
      (else
        (set `self.Movement` 200.0)
        (goto _label_2)))
    (elif (== _returnvalue 2)
      (goto _label)
      (else
        (set `self.Movement` 200.0)
        (goto _label_2)))))

(event `Move Clone`
  (bind _returnvalue_x (`KismetMathLibrary.BreakVector` (`self.K2_GetActorLocation`)))
  (bind (_returnvalue_x_2 _returnvalue_y) (`KismetMathLibrary.BreakVector` (`self.K2_GetActorLocation`)))
  (bind _returnvalue (+ _returnvalue_y (`self.Movement`)))
  (bind _returnvalue_2 (+ _returnvalue_x (`self.Movement`)))
  (if (`self.Up`)
    (if (or (< _returnvalue (`self.MinimumY`)) (> _returnvalue (`self.Maximum Y`)))
      (`self.Where to move?` :!label _label_3)
      (else
        (set `self.LocY` _returnvalue)
        (`self.K2_TeleportTo` (`KismetMathLibrary.MakeVector` (`self.LocX`) (`self.LocY`)) :!label _label_4)
        (`KismetSystemLibrary.Delay` 0.75)
        (`self.Where to move?`)))
    (elif (or (< _returnvalue_2 (`self.MinimumX`)) (> _returnvalue_2 (`self.Maximum X`)))
      (goto _label_3)
      (else
        (set `self.LocX` _returnvalue_2)
        (goto _label_4)))))

(event `self.ReceiveAnyDamage`
  (params (Damage :type "Float (single-precision)") (DamageType :type "DamageType Object Reference") (InstigatedBy :type "Controller Object Reference") (DamageCauser :type "Actor Object Reference"))
  (bind _output_get (set `self.Life` (- (`self.Life`) Damage)))
  (`KismetSystemLibrary.PrintString` (`KismetStringLibrary.Conv_DoubleToString` _output_get) true true (struct :`G` 0.66 :`B` 1.0 :`A` 1.0) 5.0))

(fn `UserConstructionScript`)