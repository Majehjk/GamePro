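; Ability actor that takes on the look of a player ability by swapping its static mesh from an array.
; AxAttack plays a timeline that moves the actor along an X/Z arc offset from the first Player's SpawnLocation while pitching the mesh.
; A delay started from the timeline update destroys the actor about two seconds later.
; ShadowClone only sets its mesh, with no further behavior.
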(event `Ax Attack`
  (`StaticMeshComponent.SetStaticMesh` (`self.StaticMesh`) (`|GetArrayItem` (`self.Ability Mesh`)))
  (bind _outactors (`GameplayStatics.GetAllActorsOfClass` "/Game/Game/Blueprints/Player/Player.Player_C"))
  (bind (_direction _location__x_ _arch__z_ _rotation__y_) (`Timeline|Ax Movement`)
    (:`Update`
      (bind (_spawn_location_x _spawn_location_y _spawn_location_z) (`KismetMathLibrary.BreakVector` (`/Game/Game/Blueprints/Player/Player.Spawn Location` (`|GetArrayItem` _outactors))))
      (`SceneComponent.K2_SetWorldLocation` (`self.DefaultSceneRoot`) (`KismetMathLibrary.MakeVector` (`KismetMathLibrary.Lerp` 0.0 (+ _location__x_ _spawn_location_x) 1.0) _spawn_location_y (`KismetMathLibrary.Lerp` 0.0 (+ _arch__z_ _spawn_location_z) 1.0)) false false)
      (`SceneComponent.K2_SetWorldRotation` (`self.StaticMesh`) (`KismetMathLibrary.MakeRotator` 0.0 (`KismetMathLibrary.Lerp` 0.0 _rotation__y_ 1.0)) false false)
      (`KismetSystemLibrary.Delay` 2.0)
      (`self.K2_DestroyActor`))))

(event `ShadowClone`
  (`StaticMeshComponent.SetStaticMesh` (`self.StaticMesh`) (`|GetArrayItem` (`self.Ability Mesh`) 1)))

(fn `UserConstructionScript`)