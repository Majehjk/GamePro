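; Ability actor for the player Knth, providing an Intel Wall and an Angel Shield.
; Each ability event adds a static mesh, then issues an AI move on the player pawn's controller toward a fixed offset from the stored player location (sideways for the wall, overhead for the shield).
; Life checks destroy the actor immediately at zero life, otherwise after a short delay; the shield's check runs on Tick behind a gate.
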(event `self.ReceiveBeginPlay`
  (bind _asplayer (cast `/Game/Game/Blueprints/Player/Player` (`GameplayStatics.GetPlayerCharacter` 0)))
  (set `self.boplayer` _asplayer))

(event `Intel_Wall`
  ;[1 1 1] WallLife1
  (`AddComponent|NODE_AddStaticMeshComponent-2` :`RelativeTransform` (`self.GetTransform`))
  (`AITask_MoveTo.AIMoveTo` (`AIBlueprintHelperLibrary.GetAIController` (`GameplayStatics.GetPlayerPawn` 0)) (+ (`/Game/Game/Blueprints/Player/Player.PlayerLocation` (`self.boplayer`)) (0.0 349.0 0.0))
    (:`then`
      (`self.Wall_Lifee`))))

(event `Wall_Lifee`
  ;[1 1 1] WallLife1
  (if (<= (`self.Wall_LIfe`) 0.0)
    (`self.K2_DestroyActor`)
    (else
      (`KismetSystemLibrary.Delay` 2.0)
      (`self.K2_DestroyActor`))))

(event `AngelShield`
  ;[0 0.8448 1] AngelShield
  (`AddComponent|NODE_AddStaticMeshComponent-0` :`RelativeTransform` (`self.GetTransform`))
  (`AITask_MoveTo.AIMoveTo` (`AIBlueprintHelperLibrary.GetAIController` (`GameplayStatics.GetPlayerPawn` 0)) (+ (`/Game/Game/Blueprints/Player/Player.PlayerLocation` (`self.boplayer`)) (0.0 0.0 400.0))
    (:`then`
      (`self.Angel_Life`))))

(event `self.ReceiveTick`
  (params (DeltaSeconds :type "Float (single-precision)"))
  ;[0 0.8448 1] AngelShield
  (`/Engine/EditorBlueprintResources/StandardMacros.Gate` true :!label _label
    (:`Exit`
      (if (<= (`self.Shield_Life`) 0.0)
        (`self.K2_DestroyActor`)
        (else
          (`KismetSystemLibrary.Delay` 2.0)
          (`self.K2_DestroyActor`))))))

(event `Angel_Life`
  ;[0 0.8448 1] AngelShield
  (goto _label :!via `Open`))

(fn `UserConstructionScript`)