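; Ability actor that runs one of five named player abilities through Activate.
; Axe arcs a spinning mesh from the player's spawn location, Fire slides a mesh then adds another ahead, and Lightning grows a capsule collision forward; Cannon and Water delegate to Player functions.
; Timelines drive the motion; those three abilities destroy the actor after delays, with Fire resetting the player's tile and Lightning restoring input and movement.
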(event `self.ReceiveBeginPlay`
  ;[1 1 1] Begin Play / Cast to Player
  (bind _asplayer (cast `/Game/Game/Blueprints/Player/Player` (`GameplayStatics.GetPlayerCharacter` 0)))
  (set `self.Player` _asplayer))

(event `InfinteLaser`
  (bind _lasercollision (`self.LaserCollision`))
  ;[0.6003 0.3001 1] Laser Collision / Scales up and moves
  (bind _returnvalue (`AddComponent|NODE_AddCapsuleComponent-0` :`RelativeTransform` (`KismetMathLibrary.MakeTransform` (0.0 0.0 0.0) (struct :`Pitch` 90.0))))
  (set `self.LaserCollision` _returnvalue)
  (`Timeline|Timeline_0`
    (:`Update`
      (`SceneComponent.SetRelativeScale3D` _lasercollision (+ (`SceneComponent.RelativeScale3D` _returnvalue) (0.0 0.0 0.5)))
      (`SceneComponent.K2_SetRelativeLocation` _lasercollision (+ (`SceneComponent.RelativeLocation` _returnvalue) (22.5 0.0 0.0)) false false)
      (`KismetSystemLibrary.Delay` 1.0)
      (`self.EnableInput` (`self.Player`) (`GameplayStatics.GetPlayerController` 0))
      (set `/Game/Game/Blueprints/Player/Player.MovementEnable` true (`self.Player`))
      (`self.K2_DestroyActor`))))

(event `Activate`
  (params (Name :type Text))
  (bind _player (`self.Player`))
  (switch `string` (`KismetTextLibrary.Conv_TextToString` Name)
    (:`Axe`
      (`self.Ax Attack`))
    (:`Cannon`
      (`/Game/Game/Blueprints/Player/Player.Lane` _player))
    (:`Fire`
      (`self.TwoTileSpread`))
    (:`Lightning`
      (`self.InfinteLaser`))
    (:`Water`
      (`/Game/Game/Blueprints/Player/Player.Clone` _player))))

(event `TwoTileSpread`
  (`StaticMeshComponent.SetStaticMesh` (`self.Spawn`) (`|GetArrayItem` (`self.AbilityObjects`)))
  (set `self.TwoTileLoc` (`SceneComponent.K2_GetComponentLocation` (`self.Spawn`)))
  (bind (_direction _location_x) (`Timeline|Timeline_1` :`NewTime` 0.0)
    (:`Update`
      (bind _output_get (set `self.NewTwoTileLoc` (+ (`self.TwoTileLoc`) _location_x)))
      (`SceneComponent.K2_SetWorldLocation` (`self.Spawn`) _output_get false false)
      (`KismetSystemLibrary.Delay` 2.0)
      (bind _returnvalue (`AddComponent|NODE_AddStaticMeshComponent-0`))
      (`StaticMeshComponent.SetStaticMesh` _returnvalue (`|GetArrayItem` (`self.AbilityObjects`)))
      (`SceneComponent.K2_SetWorldLocation` _returnvalue (+ (`self.NewTwoTileLoc`) (200.0 0.0 0.0)) false false)
      (`KismetSystemLibrary.Delay` 3.0)
      (`/Game/Game/Blueprints/Player/Player.ResetTtile` (`self.Player`))
      (`self.K2_DestroyActor`))))

(event `Ax Attack`
  (`StaticMeshComponent.SetStaticMesh` (`self.Spawn`) (`|GetArrayItem` (`self.AbilityObjects`) 1))
  (bind _outactors (`GameplayStatics.GetAllActorsOfClass` "/Game/Game/Blueprints/Player/Player.Player_C"))
  (bind (_direction _location__x_ _arch__z_ _rotation__y_) (`Timeline|Timeline_2`)
    (:`Update`
      (bind (_spawn_location_x _spawn_location_y _spawn_location_z) (`KismetMathLibrary.BreakVector` (`/Game/Game/Blueprints/Player/Player.Spawn Location` (`|GetArrayItem` _outactors))))
      (`SceneComponent.K2_SetWorldLocation` (`self.DefaultSceneRoot`) (`KismetMathLibrary.MakeVector` (`KismetMathLibrary.Lerp` 0.0 (+ _location__x_ _spawn_location_x) 1.0) _spawn_location_y (`KismetMathLibrary.Lerp` 0.0 (+ _arch__z_ _spawn_location_z) 1.0)) false false)
      (`SceneComponent.K2_SetWorldRotation` (`self.Spawn`) (`KismetMathLibrary.MakeRotator` 0.0 (`KismetMathLibrary.Lerp` 0.0 _rotation__y_ 1.0)) false false)
      (`KismetSystemLibrary.Delay` 2.0)
      (`self.K2_DestroyActor`))))

(fn `UserConstructionScript`)