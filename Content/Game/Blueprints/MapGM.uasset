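; MapGM is a multiplayer game mode that spawns and possesses a Player pawn at successive TargetPoints for each login.
; After a short delay, it switches all tracked players to a shared GameCamera.
; It also caches the Map_Grid, asks BP_GameInstance to destroy the session on logout, and records swapped controllers.
; The countdown's starter, main-menu setup and random PlayerStart respawn are disconnected, leaving RespawnPlayer empty.
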(event `self.K2_PostLogin`
  (params (NewPlayer :type "PlayerController Object Reference"))
  ;[1 1 1] On PostLogin / Get Target Points and spawn players / Set Cameras
  (`KismetArrayLibrary.Array_Add` (`self.AllPlayers`) NewPlayer)
  (bind _outactors (`GameplayStatics.GetAllActorsOfClass` "/Script/Engine.TargetPoint"))
  (set `self.TPoints_Ref` _outactors)
  (bind _returnvalue (`|SpawnActorFromClass` "/Game/Game/Blueprints/Player/Player.Player_C" (`self.GetTransform` (`|GetArrayItem` (`self.TPoints_Ref`) (`self.TPointIndex`))) "AlwaysSpawn" "OverrideRootScale"))
  (`Controller.Possess` NewPlayer _returnvalue)
  (`/Engine/EditorBlueprintResources/StandardMacros.IncrementInt` (`self.TPointIndex`)
    (:`  `
      (`KismetSystemLibrary.Delay` 2.0)
      (for _array_element (`self.AllPlayers`)
        (`PlayerController.SetViewTargetWithBlend` _array_element (`self.GameCamera`) 0.0 "VTBlend_Linear" 0.0 false)))))

(event `self.ReceiveBeginPlay`
  ;[1 1 1] Begin Play / Get MapGrid
  (bind _outactors (`GameplayStatics.GetAllActorsOfClass` "/Game/Game/Blueprints/Grid_Programacion/Map_Grid.Map_Grid_C"))
  (set `self.MapGrid_Ref` (`|GetArrayItem` _outactors)))

(event `Timer`
  (if (== (`self.secons`) 0)
    (`/Engine/EditorBlueprintResources/StandardMacros.DecrementInt` (`self.MIn`)
      (:`  `
        (set `self.secons` 59)))
    (else
      (`/Engine/EditorBlueprintResources/StandardMacros.DecrementInt` (`self.secons`)))))

(event `self.K2_OnLogout`
  (params (ExitingController :type "Controller Object Reference"))
  ;[1 1 1] Event OnLogout - Destroy Session Caller
  (bind _asplayer_controller (cast `PlayerController` ExitingController))
  (`/Game/Game/Blueprints/BP_GameInstance.DestroySession` (cast `/Game/Game/Blueprints/BP_GameInstance` (`GameplayStatics.GetGameInstance`) :!pure true) _asplayer_controller))

(event `self.K2_OnSwapPlayerControllers`
  (params (OldPC :type "PlayerController Object Reference") (NewPC :type "PlayerController Object Reference"))
  ;[1 1 1] Keeps Tracks of Connect Player Controller
  (`KismetArrayLibrary.Array_Add` (`self.AllPlayerCharacters`) NewPC))

(event `RespawnPlayer`
  (params (PlayerController :type "PlayerController Object Reference") (PlayerCharacter :type "Character Class Reference"))
  ;[1 0.02708 0] Spawn Player with Selected Character (POTENTIAL ERASE)
)

(fn `OnRep_MapGrid_Ref`)

(fn `OnRep_SpawnPoints`)

(fn `UserConstructionScript`)