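; Tablero is a 3x3 board actor that teleports the player character between nine tile locations with the WASD keys.
; On BeginPlay it applies one material to all floors and fills a one-based array of teleport points.
; Each tile's overlap box stores the four neighbor indices, clamped at the edges, which the key events use as destinations.
; Input is enabled only when the center box is overlapped.
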(event `color`
  (`PrimitiveComponent.SetMaterial` (`self.Floor2`) 0 (`self.NewVar_0`))
  (`PrimitiveComponent.SetMaterial` (`self.Floor3`) 0 (`self.NewVar_0`))
  (`PrimitiveComponent.SetMaterial` (`self.floor4`) 0 (`self.NewVar_0`))
  (`PrimitiveComponent.SetMaterial` (`self.Floor5`) 0 (`self.NewVar_0`))
  (`PrimitiveComponent.SetMaterial` (`self.Floor6`) 0 (`self.NewVar_0`))
  (`PrimitiveComponent.SetMaterial` (`self.Floor7`) 0 (`self.NewVar_0`))
  (`PrimitiveComponent.SetMaterial` (`self.Floor8`) 0 (`self.NewVar_0`))
  (`PrimitiveComponent.SetMaterial` (`self.Floor9`) 0 (`self.NewVar_0`))
  (`PrimitiveComponent.SetMaterial` (`self.Floor1`) 0 (`self.NewVar_0`)))

(event `self.ReceiveBeginPlay`
  ;[0 0 1] Ref De teleport
  ;;[0 1 0] EB
  (`self.color`)
  (set `self.teleport locations` (`|MakeArray` null (`self.tele1`) (`self.tele2`) (`self.tele3`) (`self.tele4`) (`self.tele5`) (`self.tele6`) (`self.tele7`) (`self.tele8`) (`self.tele9`))))

(event `Key|W`
  (params (Key :type "Key Structure" :default "AnyKey"))
  ;[1 0 0] Teleport ***Flata Botons***
  ;;[0 0 1] TeleportUp
  (:`Pressed`
    (`self.K2_TeleportTo` (`GameplayStatics.GetPlayerCharacter` 0) (`SceneComponent.K2_GetComponentLocation` (`|GetArrayItem` (`self.teleport locations`) (`self.up`))) (struct :`Yaw` -90.0))))

(event `Key|S`
  (params (Key :type "Key Structure" :default "AnyKey"))
  ;[1 0 0] Teleport ***Flata Botons***
  ;;[0 0 1] TeleportDown
  (:`Pressed`
    (`self.K2_TeleportTo` (`GameplayStatics.GetPlayerCharacter` 0) (`SceneComponent.K2_GetComponentLocation` (`|GetArrayItem` (`self.teleport locations`) (`self.down`))) (struct :`Yaw` -90.0))))

(event `Key|A`
  (params (Key :type "Key Structure" :default "AnyKey"))
  ;[1 0 0] Teleport ***Flata Botons***
  ;;[0 0 1] TeleportLeft
  (:`Pressed`
    (`self.K2_TeleportTo` (`GameplayStatics.GetPlayerCharacter` 0) (`SceneComponent.K2_GetComponentLocation` (`|GetArrayItem` (`self.teleport locations`) (`self.Left`))) (struct :`Yaw` -90.0))))

(event `Key|D`
  (params (Key :type "Key Structure" :default "AnyKey"))
  ;[1 0 0] Teleport ***Flata Botons***
  ;;[0 0 1] TeleportRight
  (:`Pressed`
    (`self.K2_TeleportTo` (`GameplayStatics.GetPlayerCharacter` 0) (`SceneComponent.K2_GetComponentLocation` (`|GetArrayItem` (`self.teleport locations`) (`self.Rigth`))) (struct :`Yaw` -90.0))))

(event `self.Box2.OnComponentBeginOverlap`
  (params (OverlappedComponent :type "PrimitiveComponent Object Reference") (OtherActor :type "Actor Object Reference") (OtherComp :type "PrimitiveComponent Object Reference") (OtherBodyIndex :type Integer) (bFromSweep :type Boolean) (SweepResult :type "HitResult Structure (by ref)"))
  ;[0 0 1] Overlad Event To Activate next teleportation Location
  (cast `/Game/ThirdPersonBP/Blueprints/ThirdPersonCharacter` OtherActor)
  (set `self.Left` 1)
  (set `self.down` 5)
  (set `self.up` 2)
  (set `self.Rigth` 3))

(event `self.Box1.OnComponentBeginOverlap`
  (params (OverlappedComponent :type "PrimitiveComponent Object Reference") (OtherActor :type "Actor Object Reference") (OtherComp :type "PrimitiveComponent Object Reference") (OtherBodyIndex :type Integer) (bFromSweep :type Boolean) (SweepResult :type "HitResult Structure (by ref)"))
  ;[0 0 1] Overlad Event To Activate next teleportation Location
  (cast `/Game/ThirdPersonBP/Blueprints/ThirdPersonCharacter` OtherActor)
  (set `self.Left` 1)
  (set `self.down` 4)
  (set `self.up` 1)
  (set `self.Rigth` 2))

(event `self.Box3.OnComponentBeginOverlap`
  (params (OverlappedComponent :type "PrimitiveComponent Object Reference") (OtherActor :type "Actor Object Reference") (OtherComp :type "PrimitiveComponent Object Reference") (OtherBodyIndex :type Integer) (bFromSweep :type Boolean) (SweepResult :type "HitResult Structure (by ref)"))
  ;[0 0 1] Overlad Event To Activate next teleportation Location
  (cast `/Game/ThirdPersonBP/Blueprints/ThirdPersonCharacter` OtherActor)
  (set `self.Left` 2)
  (set `self.down` 6)
  (set `self.up` 3)
  (set `self.Rigth` 3))

(event `self.Box4.OnComponentBeginOverlap`
  (params (OverlappedComponent :type "PrimitiveComponent Object Reference") (OtherActor :type "Actor Object Reference") (OtherComp :type "PrimitiveComponent Object Reference") (OtherBodyIndex :type Integer) (bFromSweep :type Boolean) (SweepResult :type "HitResult Structure (by ref)"))
  ;[0 0 1] Overlad Event To Activate next teleportation Location
  (cast `/Game/ThirdPersonBP/Blueprints/ThirdPersonCharacter` OtherActor)
  (set `self.Left` 4)
  (set `self.down` 7)
  (set `self.up` 1)
  (set `self.Rigth` 5))

(event `self.Box6.OnComponentBeginOverlap`
  (params (OverlappedComponent :type "PrimitiveComponent Object Reference") (OtherActor :type "Actor Object Reference") (OtherComp :type "PrimitiveComponent Object Reference") (OtherBodyIndex :type Integer) (bFromSweep :type Boolean) (SweepResult :type "HitResult Structure (by ref)"))
  ;[0 0 1] Overlad Event To Activate next teleportation Location
  (cast `/Game/ThirdPersonBP/Blueprints/ThirdPersonCharacter` OtherActor)
  (set `self.Left` 5)
  (set `self.down` 9)
  (set `self.up` 3)
  (set `self.Rigth` 6))

(event `self.Box5.OnComponentBeginOverlap`
  (params (OverlappedComponent :type "PrimitiveComponent Object Reference") (OtherActor :type "Actor Object Reference") (OtherComp :type "PrimitiveComponent Object Reference") (OtherBodyIndex :type Integer) (bFromSweep :type Boolean) (SweepResult :type "HitResult Structure (by ref)"))
  ;[0 0 1] Overlad Event To Activate next teleportation Location
  (`self.EnableInput` (`GameplayStatics.GetPlayerController` 0))
  (cast `/Game/ThirdPersonBP/Blueprints/ThirdPersonCharacter` OtherActor)
  (set `self.Left` 4)
  (set `self.down` 8)
  (set `self.up` 2)
  (set `self.Rigth` 6))

(event `self.Box9.OnComponentBeginOverlap`
  (params (OverlappedComponent :type "PrimitiveComponent Object Reference") (OtherActor :type "Actor Object Reference") (OtherComp :type "PrimitiveComponent Object Reference") (OtherBodyIndex :type Integer) (bFromSweep :type Boolean) (SweepResult :type "HitResult Structure (by ref)"))
  ;[0 0 1] Overlad Event To Activate next teleportation Location
  (cast `/Game/ThirdPersonBP/Blueprints/ThirdPersonCharacter` OtherActor)
  (set `self.Left` 8)
  (set `self.down` 9)
  (set `self.up` 6)
  (set `self.Rigth` 9))

(event `self.Box8.OnComponentBeginOverlap`
  (params (OverlappedComponent :type "PrimitiveComponent Object Reference") (OtherActor :type "Actor Object Reference") (OtherComp :type "PrimitiveComponent Object Reference") (OtherBodyIndex :type Integer) (bFromSweep :type Boolean) (SweepResult :type "HitResult Structure (by ref)"))
  ;[0 0 1] Overlad Event To Activate next teleportation Location
  (cast `/Game/ThirdPersonBP/Blueprints/ThirdPersonCharacter` OtherActor)
  (set `self.Left` 7)
  (set `self.down` 8)
  (set `self.up` 5)
  (set `self.Rigth` 9))

(event `self.Box7.OnComponentBeginOverlap`
  (params (OverlappedComponent :type "PrimitiveComponent Object Reference") (OtherActor :type "Actor Object Reference") (OtherComp :type "PrimitiveComponent Object Reference") (OtherBodyIndex :type Integer) (bFromSweep :type Boolean) (SweepResult :type "HitResult Structure (by ref)"))
  ;[0 0 1] Overlad Event To Activate next teleportation Location
  (cast `/Game/ThirdPersonBP/Blueprints/ThirdPersonCharacter` OtherActor)
  (set `self.Left` 7)
  (set `self.down` 7)
  (set `self.up` 4)
  (set `self.Rigth` 8))

(fn `UserConstructionScript`)