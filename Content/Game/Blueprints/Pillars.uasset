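; Decorative-style pillar actor that continuously bobs slightly up and down while rotating.
; BeginPlay assigns the mesh from Pilars and starts MoveUpDown, where a FlipFlop alternates the UpDown timeline between play and reverse, re-triggering itself on Finished.
; The timeline lerps the mesh's relative Z position, while Tick adds a fixed world rotation each frame, making spin speed frame-rate dependent.
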(event `self.ReceiveBeginPlay`
  (`StaticMeshComponent.SetStaticMesh` (`self.Pilar`) (`self.Pilars`))
  (`self.moveUpDown`))

(event `moveUpDown`
  (`/Engine/EditorBlueprintResources/StandardMacros.FlipFlop`
    (:`A`
      (bind (_direction _float) (`Timeline|UpDown` :!label _label)
        (:`Update`
          (`SceneComponent.K2_SetRelativeLocation` (`self.Pilar`) (`KismetMathLibrary.VLerp` (0.0 0.0 10.0) (0.0 0.0 11.5) _float) false false))
        (:`Finished`
          (`self.moveUpDown`))))
    (:`B`
      (goto _label :!via `ReverseFromEnd`))))

(event `self.ReceiveTick`
  (params (DeltaSeconds :type "Float (single-precision)"))
  (`SceneComponent.K2_AddWorldRotation` (`self.Pilar`) (struct :`Yaw` 0.5) false false))

(fn `UserConstructionScript`)